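; BP_Player is the player Blueprint that manages the HUD and controls-info widgets.
; On BeginPlay it creates both widgets, adds them to the viewport and hides them.
; ShowUI refreshes and reveals the HUD, and HideUI hides it.
; The I key and ShowInfoUI event toggle the controls panel through ShowInfoControls, while Escape hides it.
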(event `self.ReceiveBeginPlay`
  (bind _returnvalue (`|CreateWidget` "/Game/UI/WB_HUD.WB_HUD_C"))
  (`UserWidget.AddToViewport` _returnvalue 0)
  (set `self.Hud` _returnvalue)
  (`Widget.SetVisibility` (`self.Hud`) "Hidden")
  (bind _returnvalue_2 (`|CreateWidget` "/Game/UI/WB_InfoControls.WB_InfoControls_C"))
  (bind _output_get (set `self.InfoControls` _returnvalue_2))
  (`UserWidget.AddToViewport` _output_get 0)
  (`Widget.SetVisibility` (`self.InfoControls`) "Hidden"))

(event `Key|I`
  (params (Key :type "Key Structure"))
  (:`Pressed`
    (`self.ShowInfoControls`)))

(event `self.ShowUI`
  (bind _hud (`self.Hud`))
  (`/Game/UI/WB_HUD.UpdateUI` _hud)
  (set `Widget.Visibility` "Visible" _hud))

(event `self.HideUI`
  (set `Widget.Visibility` "Hidden" (`self.Hud`)))

(event `Key|Escape`
  (params (Key :type "Key Structure"))
  (:`Pressed`
    (`Widget.SetVisibility` (`self.InfoControls`) "Hidden")))

(event `self.ShowInfoUI`
  (`self.ShowInfoControls`))

(fn `ShowInfoControls`
  (if (`|EnumEquality` (`Widget.Visibility` (`self.InfoControls`)) "Visible")
    (`Widget.SetVisibility` (`self.InfoControls`) "Hidden")
    (else
      (`Widget.SetVisibility` (`self.InfoControls`) "Visible"))))

(fn `UserConstructionScript`)