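; BP_PlantObstacle is a plant obstacle actor that displays a vulnerability sign through a widget component.
; On BeginPlay it sets itself as the owning actor of the WB_VulnerabilitySign widget and turns off the widget's shadow casting.
; Every Tick it rotates the widget to face player 0's camera, billboard style.
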(event `self.ReceiveBeginPlay`
  (bind _aswb_vulnerability_sign (cast `/Game/UI/WB_VulnerabilitySign` (`WidgetComponent.GetWidget` (`self.Widget`))))
  (set `/Game/UI/WB_VulnerabilitySign.OwningActor` self _aswb_vulnerability_sign)
  (`PrimitiveComponent.SetCastShadow` (`self.Widget`) false))

(event `self.ReceiveTick`
  (params (DeltaSeconds :type "Float (single-precision)"))
  (bind _widget (`self.Widget`))
  (`SceneComponent.K2_SetWorldRotation` _widget (`KismetMathLibrary.FindLookAtRotation` (`SceneComponent.K2_GetComponentLocation` _widget) (`SceneComponent.K2_GetComponentLocation` (`PlayerCameraManager.TransformComponent` (`GameplayStatics.GetPlayerCameraManager` 0)))) false false))

(fn `UserConstructionScript`)