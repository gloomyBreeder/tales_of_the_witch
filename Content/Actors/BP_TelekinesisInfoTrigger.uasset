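; BP_TelekinesisInfoTrigger is a one-time hint trigger that shows telekinesis info text when the player enters its box.
; Overlap shows a widget with either the Q key prompt or a heavy-stones hint, depending on the player's CanTelekinesis result, and hides it on exit.
; Tick watches for an overlapping, capable player entering telekinesis, then clears a flag so the actor destroys itself the following tick.
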(event `self.ReceiveBeginPlay`
  (`SceneComponent.SetVisibility` (`self.Widget`) false false)
  (add `PrimitiveComponent.OnComponentBeginOverlap` (`self.Box`) (delegate `OnComponentBeginOverlap_Event`))
  (add `PrimitiveComponent.OnComponentEndOverlap` (`self.Box`) (delegate `OnComponentEndOverlap_Event`))
  (set `self.NeedShowText` true))

(event `OnComponentBeginOverlap_Event`
  (params (OverlappedComponent :type "PrimitiveComponent Object Reference") (OtherActor :type "Actor Object Reference") (OtherComp :type "PrimitiveComponent Object Reference") (OtherBodyIndex :type Integer) (bFromSweep :type Boolean) (SweepResult :type "HitResult Structure (by ref)"))
  (if (not (`self.IsOverlapping`))
    (bind _asbp_player (cast `/Game/Player/BP_Player` OtherActor))
    (`/Engine/EditorBlueprintResources/StandardMacros.IsValid` _asbp_player
      (:`Is Valid`
        (set `self.Player` _asbp_player)
        (set `self.IsOverlapping` true)
        (bind _returnvalue (`InputCharacter.CanTelekinesis` _asbp_player))
        (if _returnvalue
          (set `self.CheckCondition` true)
          (bind _aswb_info_text (cast `/Game/UI/WB_InfoText` (`WidgetComponent.GetWidget` (`self.Widget`))))
          (`TextBlock.SetText` (`/Game/UI/WB_InfoText.TextInfo` _aswb_info_text) "Press Q for telekinesis")
          (else
            (bind _aswb_info_text_2 (cast `/Game/UI/WB_InfoText` (`WidgetComponent.GetWidget` (`self.Widget`))))
            (`TextBlock.SetText` (`/Game/UI/WB_InfoText.TextInfo` _aswb_info_text_2) "The stones are very heavy. You need to figure out how to move them away")))
        (`SceneComponent.SetVisibility` (`self.Widget`) true false)))))

(event `OnComponentEndOverlap_Event`
  (params (OverlappedComponent :type "PrimitiveComponent Object Reference") (OtherActor :type "Actor Object Reference") (OtherComp :type "PrimitiveComponent Object Reference") (OtherBodyIndex :type Integer))
  (if (`self.IsOverlapping`)
    (bind _asbp_player (cast `/Game/Player/BP_Player` OtherActor))
    (`/Engine/EditorBlueprintResources/StandardMacros.IsValid` _asbp_player
      (:`Is Valid`
        (set `self.Player` null)
        (set `self.IsOverlapping` false)
        (`KismetSystemLibrary.PrintString` "end overlap")
        (`SceneComponent.SetVisibility` (`self.Widget`) false false)))))

(event `self.ReceiveTick`
  (params (DeltaSeconds :type "Float (single-precision)"))
  (bind _player (`self.Player`))
  (if (`self.NeedShowText`)
    (if (and (`self.IsOverlapping`) (`self.CheckCondition`))
      (`/Engine/EditorBlueprintResources/StandardMacros.IsValid` _player
        (:`Is Valid`
          (bind _returnvalue (`InputCharacter.IsInTelekinesis` _player))
          (if _returnvalue
            (set `self.NeedShowText` false)))))
    (else
      (`self.K2_DestroyActor`))))

(fn `UserConstructionScript`)