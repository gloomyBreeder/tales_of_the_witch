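; BP_DialogueManager is an actor that shows and hides the on-screen dialogue window.
; On BeginPlay it creates a WB_DialogueWindow for the first player controller, adds it to the viewport and keeps it hidden.
; OpenDialogue reveals the window and passes it the text, while CloseDialogue hides and clears it.
; IsTyping reports the widget's TextIsTyping state, returning false if the widget is invalid.
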(event `self.ReceiveBeginPlay`
  (bind _returnvalue (`|CreateWidget` "/Game/UI/WB_DialogueWindow.WB_DialogueWindow_C" (`GameplayStatics.GetPlayerController` 0)))
  (bind _output_get (set `self.DialogueWindow` _returnvalue))
  (`UserWidget.AddToViewport` _output_get 0)
  (set `Widget.Visibility` "Hidden" _output_get))

(event `self.OpenDialogue`
  (params (Text :type "Text (by ref)"))
  (bind _dialoguewindow (`self.DialogueWindow`))
  (set `Widget.Visibility` "Visible" _dialoguewindow)
  (`/Game/UI/WB_DialogueWindow.UpdateText` _dialoguewindow (`KismetTextLibrary.Conv_TextToString` Text)))

(event `self.CloseDialogue`
  (bind _dialoguewindow (`self.DialogueWindow`))
  (set `Widget.Visibility` "Hidden" _dialoguewindow)
  (`/Game/UI/WB_DialogueWindow.ClearText` _dialoguewindow))

(fn `IsTyping`
  (returns (ReturnValue :type Boolean))
  (bind _dialoguewindow (`self.DialogueWindow`))
  (`/Engine/EditorBlueprintResources/StandardMacros.IsValid` _dialoguewindow
    (:`Is Valid`
      (return (`/Game/UI/WB_DialogueWindow.TextIsTyping` _dialoguewindow)))
    (:`Is Not Valid`
      (return false))))

(fn `UserConstructionScript`)