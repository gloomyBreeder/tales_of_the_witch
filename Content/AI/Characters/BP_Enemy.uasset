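; BP_Enemy is an enemy character Blueprint that carries a health bar widget component named Hud.
; On BeginPlay it casts the Hud widget to WB_HealthBar, sets itself as that widget's owning actor and turns off shadow casting on Hud.
; Every Tick it billboards Hud by rotating it toward the player camera manager's location.
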(event `self.ReceiveBeginPlay`
  (bind _aswb_health_bar (cast `/Game/UI/WB_HealthBar` (`WidgetComponent.GetWidget` (`self.Hud`))))
  (set `/Game/UI/WB_HealthBar.OwningActor` self _aswb_health_bar)
  (`PrimitiveComponent.SetCastShadow` (`self.Hud`) false))

(event `self.ReceiveTick`
  (params (DeltaSeconds :type "Float (single-precision)"))
  (bind _hud (`self.Hud`))
  (`SceneComponent.K2_SetWorldRotation` _hud (`KismetMathLibrary.FindLookAtRotation` (`SceneComponent.K2_GetComponentLocation` _hud) (`SceneComponent.K2_GetComponentLocation` (`PlayerCameraManager.TransformComponent` (`GameplayStatics.GetPlayerCameraManager` 0)))) false false))

(fn `UserConstructionScript`)